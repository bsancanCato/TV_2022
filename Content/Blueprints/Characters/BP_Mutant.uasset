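; BP_Mutant is an enemy character with melee attack data and a ranged fireball attack aimed at the player.
; DañoRecibido subtracts damage from VidaMaxima and destroys the actor when it would reach zero.
; FireBalls spawns BP_FireBall from a head point toward the player, throttled by a DoOnce that resets after a short delay.
; Getter functions supply left-hand hitbox endpoints, damage and Swiping or Roaring montages, while IniciaHit and FinHit are empty.
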(event Custom|FireBalls
  (bind _scene_head_ini (Variables|Default|GetScene_Head_Ini))
  (bind _returnvalue (Transformation|GetWorldLocation _scene_head_ini))
  (Utilities|FlowControl|DoOnce false :!label _label
    (:Completed
      (Game|SpawnActorfromClass "/Game/Blueprints/Ataques/BP_FireBall.BP_FireBall_C" (Math|Transform|MakeTransform _returnvalue (Math|Rotator|FindLookatRotation _returnvalue (Transformation|GetActorLocation (Game|GetPlayerCharacter 0))) "2.000000,2.000000,2.000000") "AdjustIfPossibleButAlwaysSpawn" 0 4e+03 4.0 0)
      (Utilities|FlowControl|Delay 0.2)
      (goto _label Reset))))

(event EventBeginPlay)

(event Collision|EventActorBeginOverlap
  (params (OtherActor :type Actor%20Object%20Reference)))

(event EventTick
  (params (DeltaSeconds :type Float%20%28single-precision%29)))

(event EventDañoRecibido
  (params (Valor :type Integer))
  (if (> (- (Variables|Parametros|GetVidaMaxima) Valor) 0)
    (Variables|Parametros|SetVidaMaxima (- (Variables|Parametros|GetVidaMaxima) Valor))
    (else
      (Actor|DestroyActor))))

(fn ConstructionScript)

(fn IniciaHit)

(fn FinHit)

(fn GetAtaqueEspecial
  (params (Ataque :type E_Ataques%20Enum :default "NewEnumerator0"))
  (switch Utilities|FlowControl|Switch|SwitchonE_Ataques Ataque
    (:NewEnumerator0
      (return "/Game/Characters/Mutant/Animaciones/AM_Swiping.AM_Swiping"))
    (:NewEnumerator1
      (return "/Game/Characters/Mutant/Animaciones/AM_Roaring.AM_Roaring"))))

(fn GetHitBoxFin
  (return (Transformation|GetWorldLocation (Variables|Default|GetScene_LeftHand_Fin))))

(fn GetHitBoxInicio
  (return (Transformation|GetWorldLocation (Variables|Default|GetScene_LeftHand_Ini))))

(fn GetValorDaño
  (return 10))