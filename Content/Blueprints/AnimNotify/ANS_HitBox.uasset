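; Anim notify state that acts as a melee-style hit box, dealing damage while its window in an animation is active.
; Each tick, it gets start and end points from the mesh owner through IHitBox and sphere-traces between them on the Camera channel.
; A hit actor implementing IRecibirDaño receives the owner's damage value.
; Hit actors are not tracked, so one target can be damaged on successive ticks.
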(fn ReceivedNotifyTick
  (params (MeshComp :type Skeletal%20Mesh%20Component%20Object%20Reference) (Animation :type Anim%20Sequence%20Base%20Object%20Reference) (FrameDeltaTime :type Float%20%28single-precision%29) (EventReference :type Anim%20Notify%20Event%20Reference%20Structure%20%28by%20ref%29))
  (bind _returnvalue (Components|GetOwner MeshComp))
  (if (Utilities|DoesObjectImplementInterface _returnvalue "/Game/Blueprints/Interface/IHitBox.IHitBox_C")
    (bind _posicion (Class|IHitBox|GetHitBoxInicio(Message) _returnvalue))
    (bind _posicion_2 (Class|IHitBox|GetHitBoxFin(Message) _returnvalue))
    (bind _outhit (Collision|SphereTraceByChannel _returnvalue _posicion _posicion_2 5e+01 "TraceTypeQuery2" false 0 "None"))
    (if (Utilities|DoesObjectImplementInterface (.HitActor (Collision|BreakHitResult _outhit)) "/Game/Blueprints/Interface/IRecibirDaño.IRecibirDaño_C")
      (bind _valor (Class|IHitBox|GetValorDaño(Message) _returnvalue))
      (Class|IRecibirDaño|DañoRecibido(Message) (.HitActor (Collision|BreakHitResult _outhit)) _valor)
      (return true)
      (else
        (return true)))
    (else
      (return true))))