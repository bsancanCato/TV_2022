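; Basic AI pawn blueprint that chases a pawn it sees and then returns to where it started.
; BeginPlay stores the start location, and PawnSensing's OnSeePawn event issues an AI MoveTo toward the seen pawn.
; On success it sets a TargetAlcanzado flag, which ignores further sightings while it moves back to the stored location.
; Reaching the start clears the flag, and failed moves have no handling.
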(event OnSeePawn(PawnSensing)
  (params (Pawn :type Pawn%20Object%20Reference))
  (if (not (Variables|Default|GetTargetAlcanzado))
    (AI|AIMoveTo self "0, 0, 0" Pawn 5.0 false
      (:OnSuccess
        (Variables|Default|SetTargetAlcanzado true)
        (Development|PrintString "Target alcanzado")
        (AI|AIMoveTo self (Variables|Default|GetPosicionInicial) 0 5.0 false
          (:OnSuccess
            (Variables|Default|SetTargetAlcanzado false)
            (Development|PrintString "Posicion Inicial alcanzada")))))))

(event EventBeginPlay
  (Variables|Default|SetPosicionInicial (Transformation|GetActorLocation)))

(event Collision|EventActorBeginOverlap
  (params (OtherActor :type Actor%20Object%20Reference)))

(event EventTick
  (params (DeltaSeconds :type Float%20%28single-precision%29)))

(fn ConstructionScript)