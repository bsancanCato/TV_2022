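; Kamikaze AI enemy that chases the player and blows itself up when close.
; PawnSensing triggers AI Move To toward the player character; on arrival it sets a reached flag and waits briefly.
; It then explodes with particles and sound and destroys itself if the player is still near, otherwise clears the flag and resumes pursuit without needing sight.
; The explosion applies no damage here.
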(event OnSeePawn(PawnSensing)
  (params (Pawn :type Pawn%20Object%20Reference))
  (if (not (Variables|Default|GetTargetAlcanzado))
    (AI|AIMoveTo self "0, 0, 0" (Game|GetPlayerCharacter 0) 5.0 false
      (:OnSuccess
        (Variables|Default|SetTargetAlcanzado true)
        (Development|PrintString "Target alcanzado")
        (Utilities|FlowControl|Delay 1.0)
        (if (> (Transformation|GetDistanceTo self (Game|GetPlayerCharacter 0)) 5e+02)
          ;[1 1 1] Si la distancia es mayor a lo evaluado se le indica al kamikaze que persiga al player aunque no se encuentre en su rango de vision
          (Variables|Default|SetTargetAlcanzado false)
          (AI|AIMoveTo self "0, 0, 0" (Game|GetPlayerCharacter 0) 5.0 false)
          (else
            ;[1 1 1] Si la distancia es menor a la evaluada el Kamizase procede a destruirse
            (Effects|SpawnEmitteratLocation "/Game/StarterContent/Particles/P_Explosion.P_Explosion" (Transformation|GetActorLocation) "0, 0, 0" "5.000000,5.000000,5.000000")
            (Audio|PlaySoundatLocation "/Game/StarterContent/Audio/Explosion02.Explosion02" (Transformation|GetActorLocation) "0, 0, 0" 1.0 1.0 0.0 0 0 0 0)
            (Actor|DestroyActor)))))))

(event EventBeginPlay)

(event Collision|EventActorBeginOverlap
  (params (OtherActor :type Actor%20Object%20Reference)))

(event EventTick
  (params (DeltaSeconds :type Float%20%28single-precision%29)))

(fn ConstructionScript)