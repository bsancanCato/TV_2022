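; BP_Npc_AiController is the AI controller for BP_Npc_AI characters, handling their behavior tree and player detection.
; On possess it caches the NPC and runs the behavior tree assigned on that character.
; AI Perception updates write a sensed BP_ThirdPersonCharacter to the blackboard target key.
; A lost stimulus or any other actor's update clears that key, even if the player was the current target.
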(event OnTargetPerceptionUpdated(AIPerception)
  (params (Actor :type Actor%20Object%20Reference) (Stimulus :type AI%20Stimulus%20Structure))
  (if (.bSuccessfullySensed (Utilities|Struct|BreakAIStimulus Stimulus))
    (bind _asbp_third_person_character (Utilities|Casting|CastToBP_ThirdPersonCharacter Actor)
      (:then
        (CallFunction|SetTarget _asbp_third_person_character))
      (:CastFailed
        (CallFunction|SetTarget :!label _label)))
    (else
      (goto _label))))

(event EventBeginPlay)

(event EventTick
  (params (DeltaSeconds :type Float%20%28single-precision%29)))

(event EventPossess
  (params (PossessedPawn :type Pawn%20Object%20Reference))
  (bind _asbp_npc_ai (Utilities|Casting|CastToBP_Npc_AI PossessedPawn))
  (bind _output_get (Variables|Default|SetCharacterAI _asbp_npc_ai))
  (bind _behaviortree (Variables|/Game/Blueprints/Ai/Avanzado/BP_Npc_AI.BP_Npc_AI_C|GetBehaviorTree _output_get)
    (:then
      (AI|RunBehaviorTree _behaviortree))
    (:else)))

(fn ConstructionScript)

(fn SetTarget
  (params (ObjectValue :type Object%20Object%20Reference))
  (AI|Components|Blackboard|SetValueasObject (AI|GetBlackboard 0) (Variables|Default|GetTargetActorKey) ObjectValue))