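; AI controller for BP_Mutant enemies that runs their behavior tree and feeds it perceived players as targets.
; On possess, it caches the mutant and runs the BehaviorTree asset assigned on that pawn, if valid.
; AI Perception updates write successfully sensed actors tagged Player to the blackboard's target key through SetTarget.
; Losing perception does not clear the target here.
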(event OnTargetPerceptionUpdated(AIPerception)
  (params (Actor :type Actor%20Object%20Reference) (Stimulus :type AI%20Stimulus%20Structure))
  (if (Actor|ActorHasTag Actor "Player")
    (if (.bSuccessfullySensed (Utilities|Struct|BreakAIStimulus Stimulus))
      (CallFunction|SetTarget Actor))))

(event EventBeginPlay)

(event EventTick
  (params (DeltaSeconds :type Float%20%28single-precision%29)))

(event EventPossess
  (params (PossessedPawn :type Pawn%20Object%20Reference))
  (bind _asbp_mutant (Utilities|Casting|CastToBP_Mutant PossessedPawn))
  (bind _output_get (Variables|Default|SetBP_Mutant_Ref _asbp_mutant))
  (bind _behaviortree (Variables|/Game/Blueprints/Characters/BP_Mutant.BP_Mutant_C|GetBehaviorTree _output_get)
    (:then
      (AI|RunBehaviorTree _behaviortree))
    (:else)))

(fn ConstructionScript)

(fn SetTarget
  (params (ObjectValue :type Object%20Object%20Reference))
  (AI|Components|Blackboard|SetValueasObject (AI|GetBlackboard 0) (Variables|Default|GetTargetActorKey) ObjectValue))