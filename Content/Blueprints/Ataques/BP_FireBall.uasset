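; BP_FireBall is a fireball attack projectile that damages actors it overlaps.
; On BeginPlay it launches its ProjectileMovement along the forward vector at the Velocidad speed and sets its lifespan from TiempoVida.
; When its sphere overlaps an actor implementing IRecibirDaño, it sends fixed damage through that interface, spawns explosion particles and sound, then destroys itself.
; Overlaps with other actors are ignored.
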(event OnComponentBeginOverlap(Sphere)
  (params (OverlappedComponent :type Primitive%20Component%20Object%20Reference) (OtherActor :type Actor%20Object%20Reference) (OtherComp :type Primitive%20Component%20Object%20Reference) (OtherBodyIndex :type Integer) (bFromSweep :type Boolean) (SweepResult :type Hit%20Result%20Structure%20%28by%20ref%29))
  (bind _returnvalue (Transformation|GetActorLocation))
  (if (Utilities|DoesObjectImplementInterface OtherActor "/Game/Blueprints/Interface/IRecibirDaño.IRecibirDaño_C")
    (Class|IRecibirDaño|DañoRecibido(Message) OtherActor 10)
    (Effects|SpawnEmitteratLocation "/Game/StarterContent/Particles/P_Explosion.P_Explosion" _returnvalue "0, 0, 0" "1.000000,1.000000,1.000000" true "AutoRelease")
    (Audio|PlaySoundatLocation "/Game/StarterContent/Audio/Explosion01.Explosion01" _returnvalue "0, 0, 0" 1.0 1.0 0.0 0 0 0 0)
    (Actor|DestroyActor)))

(event EventBeginPlay
  ;[1 1 1] Variable para modificar la velocidad del projectile movement
  (Variables|/Script/Engine.MovementComponent|SetVelocity (Variables|Default|GetProjectileMovement) (* (Transformation|GetActorForwardVector) (Variables|Default|GetVelocidad)))
  ;[1 1 1] Variable para modificar el tiempo de vida
  (Actor|SetLifeSpan (Variables|Default|GetTiempoVida)))

(event Collision|EventActorBeginOverlap
  (params (OtherActor :type Actor%20Object%20Reference)))

(event EventTick
  (params (DeltaSeconds :type Float%20%28single-precision%29)))

(fn ConstructionScript)