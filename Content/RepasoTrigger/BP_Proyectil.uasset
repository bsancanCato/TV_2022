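; Projectile actor that damages BP_Enemigo enemies on contact.
; On BeginPlay it launches along its forward vector through ProjectileMovement and sets a short lifespan.
; Sphere overlap casts to BP_Enemigo, then either subtracts a fixed amount from VidaTotal or destroys the enemy when health would run out, printing the result.
; The projectile destroys itself after hitting an enemy; other overlaps are ignored.
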(event OnComponentBeginOverlap(Sphere)
  (params (OverlappedComponent :type Primitive%20Component%20Object%20Reference) (OtherActor :type Actor%20Object%20Reference) (OtherComp :type Primitive%20Component%20Object%20Reference) (OtherBodyIndex :type Integer) (bFromSweep :type Boolean) (SweepResult :type Hit%20Result%20Structure%20%28by%20ref%29))
  (bind _asbp_enemigo (Utilities|Casting|CastToBP_Enemigo OtherActor))
  ;[1 1 1] Se evalua si la vida que se resta sera mayor a cero. Si lo es la guardamos y actualizamos la vida del enemigo, caso contrario el enemigo sera destruido
  (if (> (- (Variables|/Game/RepasoTrigger/BP_Enemigo.BP_Enemigo_C|GetVidaTotal _asbp_enemigo) 10) 0)
    (bind _output_get (Variables|/Game/RepasoTrigger/BP_Enemigo.BP_Enemigo_C|SetVidaTotal _asbp_enemigo (- (Variables|/Game/RepasoTrigger/BP_Enemigo.BP_Enemigo_C|GetVidaTotal _asbp_enemigo) 10)))
    (Development|PrintString (Utilities|String|ToString(Integer) _output_get))
    (Actor|DestroyActor)
    (else
      (Development|PrintString "Enemigo eliminado")
      (Actor|DestroyActor _asbp_enemigo)
      (Actor|DestroyActor))))

(event EventBeginPlay
  ;[1 1 1] Variable para modificar la velocidad del projectile movement
  (Variables|/Script/Engine.MovementComponent|SetVelocity (Variables|Default|GetProjectileMovement) (* (Transformation|GetActorForwardVector) 1e+03))
  ;[1 1 1] Variable para modificar el tiempo de vida
  (Actor|SetLifeSpan 4.0))

(event Collision|EventActorBeginOverlap
  (params (OtherActor :type Actor%20Object%20Reference)))

(event EventTick
  (params (DeltaSeconds :type Float%20%28single-precision%29)))

(fn ConstructionScript)